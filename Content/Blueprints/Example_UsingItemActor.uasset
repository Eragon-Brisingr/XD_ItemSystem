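; Example actor that displays the contents of its XD inventory component as in-world text.
; Every Tick, 显示背包信息 (show inventory info) loops over the component's ItemCoreList, appends each item's name and count into one string, and writes it to a TextRender.
; NeedNotSave returns false, so the actor does not opt out of saving.
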(event EventBeginPlay)

(event Collision|EventActorBeginOverlap
  (params (OtherActor :type Actor%20Object%20Reference)))

(event EventTick
  (params (DeltaSeconds :type Float%20%28single-precision%29))
  (CallFunction|显示背包信息))

(fn ConstructionScript)

(fn 显示背包信息
  (for _array_element (Variables|/Script/XD_ItemSystem.XD_InventoryComponentBase|GetItemCoreList (Variables|Default|GetXD_InventoryComponentBase))
    (LocalVariables|Set道具信息 (Utilities|String|Append (LocalVariables|Get道具信息) (Utilities|String|ToString(Text) (Class|XDItemCoreBase|GetItemName _array_element)) "  Number  " (Utilities|String|ToString(Integer) (Variables|/Script/XD_ItemSystem.XD_ItemCoreBase|GetNumber _array_element)) " 
")))
  (Rendering|Components|TextRender|SetText (Variables|Default|GetTextRender) (Utilities|Text|ToText(String) (LocalVariables|Get道具信息))))

(fn NeedNotSave
  (return false))